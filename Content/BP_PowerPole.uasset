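; Power pole actor that strings cable components from its static mesh sockets to those of its ConnectedPole.
; RebuildPowerLine replaces existing cables, pairing sockets by index up to the smaller count and setting each cable length slightly under the socket distance.
; Construction and BeginPlay rebuild this pole and trigger rebuilds on linked poles, so lines follow edits.
; RemoveConnection destroys the spawned cables.
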(event `self.ReceiveBeginPlay`
  (bind _output (`|ConvertAsset` (`self.ConnectingPole`)))
  (bind _output_2 (`|ConvertAsset` (`self.ConnectedPole`)))
  (`self.RebuildPowerLine`)
  (`/Engine/EditorBlueprintResources/StandardMacros.IsValid` _output
    (:`Is Valid`
      (`self.RebuildPowerLine` _output))
    (:`Is Not Valid`
      _))
  (`/Engine/EditorBlueprintResources/StandardMacros.IsValid` _output_2
    (:`Is Valid`
      (`self.RebuildPowerLine` _output_2))))

(fn `RebuildPowerLine`
  (bind _returnvalue (`SceneComponent.GetAllSocketNames` (`self.StaticMesh`)))
  (bind _returnvalue_2 (`SceneComponent.GetAllSocketNames` (`/Game/BP_PowerPole.StaticMesh` (`|ConvertAsset` (`self.ConnectedPole`)))))
  (`/Engine/EditorBlueprintResources/StandardMacros.IsValid` (`|ConvertAsset` (`self.ConnectedPole`))
    (:`Is Valid`
      (for _array_element (`self.CableRef`)
        (`/Engine/EditorBlueprintResources/StandardMacros.IsValid` _array_element
          (:`Is Valid`
            (`ActorComponent.K2_DestroyComponent` _array_element))))
      (`KismetArrayLibrary.Array_Clear` (`self.CableRef`))
      (for _index (range (`KismetMathLibrary.Min` (`KismetArrayLibrary.Array_Length` _returnvalue) (`KismetArrayLibrary.Array_Length` _returnvalue_2)))
        (bind _returnvalue_3 (`SceneComponent.GetSocketLocation` (`self.StaticMesh`) (`|GetArrayItem` _returnvalue _index)))
        (bind _returnvalue_4 (`AddComponent|NODE_AddCableComponent-1` :`RelativeTransform` (`KismetMathLibrary.MakeRelativeTransform` (`KismetMathLibrary.Conv_VectorToTransform` _returnvalue_3) (`SceneComponent.GetRelativeTransform` (`self.StaticMesh`)))))
        (bind _returnvalue_5 (`SceneComponent.GetSocketLocation` (`/Game/BP_PowerPole.StaticMesh` (`|ConvertAsset` (`self.ConnectedPole`))) (`|GetArrayItem` _returnvalue_2 _index)))
        (set `CableComponent.CableLength` (* (`KismetMathLibrary.Vector_Distance` _returnvalue_3 _returnvalue_5) 0.9) _returnvalue_4)
        (`KismetArrayLibrary.Array_Add` (`self.CableRef`) _returnvalue_4)
        (set `CableComponent.EndLocation` (`KismetMathLibrary.InverseTransformLocation` (`SceneComponent.K2_GetComponentToWorld` (`self.StaticMesh`)) _returnvalue_5) _returnvalue_4)
        (`SceneComponent.K2_SetWorldLocation` _returnvalue_4 _returnvalue_3 false false)))))

(fn `RemoveConnection`
  (for _array_element (`self.CableRef`)
    (`/Engine/EditorBlueprintResources/StandardMacros.IsValid` _array_element
      (:`Is Valid`
        (`ActorComponent.K2_DestroyComponent` _array_element)))))

(fn `UserConstructionScript`
  (bind _output (`|ConvertAsset` (`self.ConnectingPole`)))
  (bind _output_2 (`|ConvertAsset` (`self.ConnectedPole`)))
  (`self.RebuildPowerLine`)
  (`/Engine/EditorBlueprintResources/StandardMacros.IsValid` _output
    (:`Is Valid`
      (`self.RebuildPowerLine` _output))
    (:`Is Not Valid`
      (`/Engine/EditorBlueprintResources/StandardMacros.IsValid` _output_2
        (:`Is Valid`
          (`self.RebuildPowerLine` _output_2))))))